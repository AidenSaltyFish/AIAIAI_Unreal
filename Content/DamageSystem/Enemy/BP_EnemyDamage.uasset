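; BP_EnemyDamage is an enemy Blueprint that can take damage and heal through a BPCDamageSystem component.
; Its health getters, Heal and TakeDamage functions forward directly to that component.
; The construction script binds events to the component's death, blocked and damage-response dispatchers.
; The Death, Blocked and DamageResponse events only print debug strings, with no gameplay reactions.
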(event Custom|Death
  (Development|PrintString "DEAD"))

(event Custom|Blocked
  (params (CanBeParried :type Boolean))
  (Development|PrintString (Utilities|String|ToString(Boolean) CanBeParried)))

(event Custom|DamageResponse
  (params (DamageResponse :type E_DamageResponse%20Enum :default "NewEnumerator0"))
  (Development|PrintString (Utilities|String|EnumtoString DamageResponse)))

(fn ConstructionScript
  (bind _bpc_damagesystem (Variables|Default|GetBPC_DamageSystem))
  (EventDispatchers|BindEventtoOnDeath _bpc_damagesystem (EventDispatchers|CreateEvent :!event Custom|Death))
  (EventDispatchers|BindEventtoOnBlocked _bpc_damagesystem (EventDispatchers|CreateEvent :!event Custom|Blocked))
  (EventDispatchers|BindEventtoOnDamageResponded _bpc_damagesystem (EventDispatchers|CreateEvent :!event Custom|DamageResponse)))

(fn GetCurHealth
  (return (Variables|/Game/DamageSystem/BPC_DamageSystem.BPC_DamageSystem_C|GetHealth (Variables|Default|GetBPC_DamageSystem))))

(fn GetMaxHealth
  (return (Variables|/Game/DamageSystem/BPC_DamageSystem.BPC_DamageSystem_C|GetMaxHealth (Variables|Default|GetBPC_DamageSystem))))

(fn Heal
  (params (Amount :type Float%20%28double-precision%29))
  (bind _updatedhealth (Default|Heal (Variables|Default|GetBPC_DamageSystem) Amount))
  (return _updatedhealth))

(fn TakeDamage
  (params (DamageInfo :type S%20Damage%20Info%20Structure))
  (bind _wasdamaged (Default|TakeDamage (Variables|Default|GetBPC_DamageSystem) DamageInfo))
  (return _wasdamaged))