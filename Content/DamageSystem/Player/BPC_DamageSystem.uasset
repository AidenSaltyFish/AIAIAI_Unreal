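; Damage system component that tracks health, death, invincibility and blocking for its owner.
; TakeDamage routes a damage info struct through CanBeDamaged to block, ignore or subtract clamped health.
; It signals blocks with the parry flag, death at zero health, and damage responses when interruptable or forced.
; Heal's clamped health logic is disconnected from its entry, so it never runs.
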(event EventBeginPlay)

(event EventTick
  (params (DeltaSeconds :type Float%20%28single-precision%29)))

(fn Heal
  (params (Amount :type Float%20%28double-precision%29)))

(fn TakeDamage
  (params (DamageInfo :type S%20Damage%20Info%20Structure))
  (bind (_amount _type _damageresponse _shoulddamageinvincible _canbeblocked _canbeparried _shouldforceinterrupt) (Utilities|Struct|BreakS_DamageInfo DamageInfo))
  (Utilities|CanbeDamaged _shoulddamageinvincible _canbeblocked
    (:BlockDamage
      (Development|PrintString "Blocked Damage")
      (Default|CallOnBlocked _canbeparried)
      (return false))
    (:DoDamage
      (bind _output_get (Variables|Default|SetHealth (Math|Float|Clamp(Float) (- (Variables|Default|GetHealth) _amount) 0.0 (Variables|Default|GetMaxHealth))))
      (bind _output_get_2 (Variables|Default|SetIsDead (<= _output_get 0.0)))
      (if _output_get_2
        (Default|CallOnDeath)
        (return true)
        (elif (or (Variables|Default|GetIsInterruptable) _shouldforceinterrupt)
          (Default|CallOnDamageResponded _damageresponse)
          (return true))))
    (:NoDamage
      (Development|PrintString "No Damage")
      (return false))))