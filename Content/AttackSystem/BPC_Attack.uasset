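; Attack component that gives its owner a homing spell, hitscan bullets, explosion, lightning strike and heal.
; MagicSpell spawns a random homing projectile that, on impact, applies damage and fires the attack-finished dispatcher; FireBullets line-traces for pawns.
; Explosion, LightningStrike and Heal spawn AOE actors at the owner and bind their overlap events to damage or healing.
; Damage and healing use interface messages; spell and bullet hits also report AI damage-sense events.
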(event Custom|HealDamage
  (params (Actor :type Actor%20Object%20Reference))
  (Class|BPIDamagable|Heal(Message) Actor (stale Custom|Heal HealAmount)))

(event Custom|OnProjectileHit
  (params (OtherActor :type Actor%20Object%20Reference) (Hit :type Hit%20Result%20Structure))
  (bind _hitactor (Collision|BreakHitResult Hit))
  (bind _returnvalue (Components|GetOwner))
  (Class|BPIDamagable|TakeDamage(Message) _hitactor (stale Custom|MagicSpell DamageInfo))
  (Class|AISenseDamage|ReportDamageEvent _hitactor _returnvalue (.Amount (Utilities|Struct|BreakS_DamageInfo (stale Custom|MagicSpell DamageInfo))) (Transformation|GetActorLocation _returnvalue) "0, 0, 0" "None")
  (Default|CallOnAttckedFinished))

(event Custom|FireBullets
  (params (TraceStart :type Vector) (TraceEnd :type Vector) (DamageInfo :type S%20Damage%20Info%20Structure))
  (bind _returnvalue (Components|GetOwner))
  (bind (_outhit _returnvalue_2) (Collision|LineTraceForObjects TraceStart TraceEnd (Utilities|Array|MakeArray "ObjectTypeQuery3") false 0 "None"))
  (if _returnvalue_2
    (Class|BPIDamagable|TakeDamage(Message) (.HitActor (Collision|BreakHitResult _outhit)) DamageInfo)
    (Class|AISenseDamage|ReportDamageEvent (.HitActor (Collision|BreakHitResult _outhit)) _returnvalue (.Amount (Utilities|Struct|BreakS_DamageInfo DamageInfo)) (Transformation|GetActorLocation _returnvalue) "0, 0, 0" "None")))

(event Custom|Explosion
  (bind _returnvalue (Game|SpawnActorfromClass "/Game/AOESystem/Blueprints/BP_AOE_Explosion.BP_AOE_Explosion_C" (Transformation|GetActorTransform (Components|GetOwner)) "Undefined" "MultiplyWithRoot" 0 0))
  (EventDispatchers|BindEventtoOnAOEOverlappedActor _returnvalue (delegate Custom|DamageExplosion)))

(event Custom|MagicSpell
  (params (SpawnTransform :type Transform) (Target :type Actor%20Object%20Reference) (DamageInfo :type S%20Damage%20Info%20Structure))
  (bind _returnvalue (Game|SpawnActorfromClass (Utilities|Select :Index (Math|Random|RandomIntegerinRange 0 2) :Option%200 "/Game/ProjectileSystem/Blueprints/BP_Projectile1.BP_Projectile1_C" :Option%201 "/Game/ProjectileSystem/Blueprints/BP_Projectile2.BP_Projectile2_C" :Option%202 "/Game/ProjectileSystem/Blueprints/BP_Projectile3.BP_Projectile3_C") SpawnTransform "Undefined" "MultiplyWithRoot" (Components|GetOwner) 5e+02 0.0 Target true 0))
  (EventDispatchers|BindEventtoOnProjectileImpact _returnvalue (delegate Custom|OnProjectileHit))
  (Collision|IgnoreActorwhenMoving (Actor|GetComponentbyClass (Components|GetOwner) "/Script/Engine.CapsuleComponent") _returnvalue true))

(event Custom|LightningStrike
  (params (Target :type Actor%20Object%20Reference) (Delay :type Float%20%28double-precision%29) (DamageAmount :type Float%20%28double-precision%29))
  (bind _returnvalue (Components|GetOwner))
  (bind _returnvalue_2 (Game|SpawnActorfromClass "/Game/AOESystem/Blueprints/BP_AOE_Lightning.BP_AOE_Lightning_C" (Transformation|GetActorTransform _returnvalue) "Undefined" "MultiplyWithRoot" _returnvalue Delay Target 0))
  (EventDispatchers|BindEventtoOnAOEOverlappedActor _returnvalue_2 (delegate Custom|DamageLightning)))

(event Custom|DamageExplosion
  (params (Actor :type Actor%20Object%20Reference))
  (Class|BPIDamagable|TakeDamage(Message) Actor (Utilities|Struct|MakeS_DamageInfo 2e+01 "NewEnumerator3")))

(event Custom|Heal
  (params (HealAmount :type Float%20%28double-precision%29))
  (bind _returnvalue (Game|SpawnActorfromClass "/Game/AOESystem/Blueprints/BP_AOE_Heal.BP_AOE_Heal_C" (Transformation|GetActorTransform (Components|GetOwner)) "Undefined" "MultiplyWithRoot" 0 0.0 0))
  (EventDispatchers|BindEventtoOnAOEOverlappedActor _returnvalue (delegate Custom|HealDamage)))

(event Custom|DamageLightning
  (params (Actor :type Actor%20Object%20Reference))
  (Class|BPIDamagable|TakeDamage(Message) Actor (Utilities|Struct|MakeS_DamageInfo (stale Custom|LightningStrike DamageAmount) "NewEnumerator2")))

(event EventBeginPlay)

(event EventTick
  (params (DeltaSeconds :type Float%20%28single-precision%29)))