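; Player character for the projectile system that fires homing projectiles, takes damage and heals.
; Q spawns a random projectile class aimed at a BP_EnemyProjectile actor, and its impact event sends damage to the hit actor.
; BPCDamageSystem handles health behind forwarding functions, feeding a widget health bar and death, block and response events.
; Death enables mesh physics and disables input, though the IsDead function always returns false.
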(event Custom|DamageEnemy
  (params (OtherActor :type Actor%20Object%20Reference) (Hit :type Hit%20Result%20Structure))
  (Class|BPIDamagable|TakeDamage(Message) (.HitActor (Collision|BreakHitResult Hit)) (Utilities|Struct|MakeS_DamageInfo 1e+01 "NewEnumerator1" "NewEnumerator1")))

(event Custom|Death
  (bind _mesh (Variables|Character|GetMesh))
  (Development|PrintString "DEAD")
  (Physics|SetSimulatePhysics _mesh true)
  (Collision|SetCollisionEnabled _mesh "QueryAndPhysics")
  (Input|DisableInput (Game|GetPlayerController 0)))

(event Custom|Blocked
  (params (CanBeParried :type Boolean))
  (Development|PrintString (Utilities|String|ToString(Boolean) CanBeParried)))

(event Custom|DamageResponse
  (params (DamageResponse :type E_DamageResponse%20Enum :default "NewEnumerator0"))
  (Development|PrintString (Utilities|String|EnumtoString DamageResponse)))

(event EventBeginPlay
  (bind _returnvalue (UserInterface|CreateWidget "/Game/DamageSystem/WBP_HealthBar.WBP_HealthBar_C" 0 self))
  (UserInterface|SetWidget (Variables|Default|GetWidget) _returnvalue))

(event Input|KeyboardEvents|Q
  (params (Key :type Key%20Structure :default "None"))
  (:Pressed
    (if (not (Variables|/Game/DamageSystem/BPC_DamageSystem.BPC_DamageSystem_C|GetIsDead (Variables|Default|GetBPC_DamageSystem)))
      (bind _returnvalue (Actor|GetActorOfClass "/Game/ProjectileSystem/Characters/BP_EnemyProjectile.BP_EnemyProjectile_C"))
      (bind _returnvalue_2 (Game|SpawnActorfromClass (Utilities|Select :Index (Math|Random|RandomIntegerinRange 0 2) :Option%200 "/Game/ProjectileSystem/Blueprints/BP_Projectile1.BP_Projectile1_C" :Option%201 "/Game/ProjectileSystem/Blueprints/BP_Projectile2.BP_Projectile2_C" :Option%202 "/Game/ProjectileSystem/Blueprints/BP_Projectile3.BP_Projectile3_C") (Transformation|GetWorldTransform (Variables|Default|GetProjectileTransform)) "Undefined" "MultiplyWithRoot" self 5e+02 0.0 _returnvalue true 0))
      (EventDispatchers|BindEventtoOnProjectileImpact _returnvalue_2 (delegate Custom|DamageEnemy))
      (Collision|IgnoreActorwhenMoving (Variables|Default|GetCapsuleComponent) _returnvalue_2 true))))

(event Input|KeyboardEvents|H
  (params (Key :type Key%20Structure :default "None"))
  (:Pressed
    (CallFunction|Heal 1e+01)))

(fn ConstructionScript
  (bind _bpc_damagesystem (Variables|Default|GetBPC_DamageSystem))
  (EventDispatchers|BindEventtoOnDeath _bpc_damagesystem (EventDispatchers|CreateEvent :!event Custom|Death))
  (EventDispatchers|BindEventtoOnBlocked _bpc_damagesystem (EventDispatchers|CreateEvent :!event Custom|Blocked))
  (EventDispatchers|BindEventtoOnDamageResponded _bpc_damagesystem (EventDispatchers|CreateEvent :!event Custom|DamageResponse)))

(fn GetCurHealth
  (return (Variables|/Game/DamageSystem/BPC_DamageSystem.BPC_DamageSystem_C|GetHealth (Variables|Default|GetBPC_DamageSystem))))

(fn GetMaxHealth
  (return (Variables|/Game/DamageSystem/BPC_DamageSystem.BPC_DamageSystem_C|GetMaxHealth (Variables|Default|GetBPC_DamageSystem))))

(fn Heal
  (params (Amount :type Float%20%28double-precision%29))
  (bind _updatedhealth (Default|Heal (Variables|Default|GetBPC_DamageSystem) Amount))
  (return _updatedhealth))

(fn IsDead
  (return false))

(fn TakeDamage
  (params (DamageInfo :type S%20Damage%20Info%20Structure))
  (bind _wasdamaged (Default|TakeDamage (Variables|Default|GetBPC_DamageSystem) DamageInfo))
  (return _wasdamaged))