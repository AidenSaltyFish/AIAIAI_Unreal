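; Base projectile actor that flies via ProjectileMovement, optionally homing on a Target, and destroys itself on hit.
; The construction script applies Speed, Gravity and homing settings to the movement component.
; BeginPlay makes the collision Box ignore the owner and aims velocity at any valid Target.
; Box hits print the component name, call OnProjectileImpact, then spawn the impact effect and sound.
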(event OnComponentHit(Box)
  (params (HitComponent :type Primitive%20Component%20Object%20Reference) (OtherActor :type Actor%20Object%20Reference) (OtherComp :type Primitive%20Component%20Object%20Reference) (NormalImpulse :type Vector :default "0, 0, 0") (Hit :type Hit%20Result%20Structure%20%28by%20ref%29))
  (bind _location (Collision|BreakHitResult Hit))
  (Development|PrintString (Utilities|GetDisplayName OtherComp))
  (Default|CallOnProjectileImpact OtherActor Hit)
  (Niagara|SpawnSystematLocation (Variables|Default|GetImpactEffect) _location)
  (Audio|PlaySoundatLocation (Variables|Default|GetImpactSound) _location "0, 0, 0" 1.0 1.0 0.0 0 0 0 0)
  (Actor|DestroyActor))

(event EventBeginPlay
  (Collision|IgnoreActorwhenMoving (Variables|Default|GetBox) (Components|GetOwner) true)
  (Variables|Default|GetTarget
    (:then
      (CallFunction|RotatetoTarget))
    (:else)))

(event Collision|EventActorBeginOverlap
  (params (OtherActor :type Actor%20Object%20Reference)))

(event EventTick
  (params (DeltaSeconds :type Float%20%28single-precision%29)))

(fn ConstructionScript
  (bind _projectilemovement (Variables|Default|GetProjectileMovement))
  (bind _speed (Variables|Default|GetSpeed))
  (Variables|/Script/Engine.ProjectileMovementComponent|SetInitialSpeed _projectilemovement _speed)
  (Variables|/Script/Engine.ProjectileMovementComponent|SetMaxSpeed _projectilemovement _speed)
  (Variables|/Script/Engine.ProjectileMovementComponent|SetProjectileGravityScale _projectilemovement (Variables|Default|GetGravity))
  (if (Variables|Default|GetIsHoming)
    (Variables|/Script/Engine.ProjectileMovementComponent|SetbIsHomingProjectile _projectilemovement true)
    (bind _target (Variables|Default|GetTarget)
      (:then
        (Variables|/Script/Engine.ProjectileMovementComponent|SetHomingTargetComponent _projectilemovement (Variables|/Script/Engine.Actor|GetRootComponent _target)))
      (:else))))

(fn RotatetoTarget
  (Variables|/Script/Engine.MovementComponent|SetVelocity (Variables|Default|GetProjectileMovement) (* (Variables|Default|GetSpeed) (Math|Vector|GetUnitDirection(Vector) (Transformation|GetActorLocation) (Transformation|GetActorLocation (Variables|Default|GetTarget))))))