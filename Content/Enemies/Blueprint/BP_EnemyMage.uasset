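; Enemy mage character with teleport and heal abilities.
; Teleport is a fast AI move in flying mode: the mesh hides, Pawn collision is ignored and fire VFX attach.
; On success or failure it restores walking, fires OnTeleportFinished and clears the effects after a short delay; repeat calls finish next tick.
; HealOverTime plays a cast montage, then calls Heal on BPCAttack with a zero amount, even if interrupted.
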(event Custom|Teleport
  (params (Destination :type Vector))
  (bind _charactermovement (Variables|Character|GetCharacterMovement))
  (if (Variables|Default|GetIsTeleporting)
    (Utilities|FlowControl|DelayUntilNextTick)
    (Default|CallOnTeleportFinished)
    (else
      (Variables|Default|SetIsTeleporting true)
      (Pawn|Components|CharacterMovement|SetMovementMode _charactermovement "MOVE_Flying" 0)
      (Variables|/Script/Engine.CharacterMovementComponent|SetMaxFlySpeed _charactermovement 5e+03)
      (Variables|/Script/Engine.CharacterMovementComponent|SetMaxAcceleration _charactermovement 1e+05)
      (Rendering|SetVisibility (Variables|Character|GetMesh) false true)
      (Collision|SetCollisionResponsetoChannel (Variables|Default|GetCapsuleComponent) "ECC_Pawn" "ECR_Ignore")
      (bind _returnvalue (Niagara|SpawnSystemAttached "/Game/MixedVFX/Particles/Fires/NS_BigFire.NS_BigFire" (Variables|Character|GetMesh) "Spine1" "0, 0, 0" "0, 0, 0" "KeepRelativeOffset" true))
      (Variables|Default|SetTeleportVFX _returnvalue)
      (bind _returnvalue_2 (Niagara|SpawnSystemAttached "/Game/MixedVFX/Particles/Fires/NS_BigFire.NS_BigFire" (Variables|Character|GetMesh) "Spine1" "0, 0, 0" "0, 0, 0" "KeepRelativeOffset" true))
      (Variables|Default|SetTrailVFX _returnvalue_2)
      (Animation|StopAnimMontage 0)
      (AI|AIMoveTo self Destination 0 15.0 false
        (:OnSuccess
          _)
        (:OnFail
          _))
      (CallFunction|TeleportFinish))))

(event Custom|TeleportFinish
  (bind _charactermovement (Variables|Character|GetCharacterMovement))
  (Components|Movement|StopMovementImmediately _charactermovement)
  (Pawn|Components|CharacterMovement|SetMovementMode _charactermovement "MOVE_Walking" 0)
  (Variables|/Script/Engine.CharacterMovementComponent|SetMaxAcceleration _charactermovement 1.5e+03)
  (Rendering|SetVisibility (Variables|Character|GetMesh) true true)
  (Collision|SetCollisionResponsetoChannel (Variables|Default|GetCapsuleComponent) "ECC_Pawn" "ECR_Block")
  (Default|CallOnTeleportFinished)
  (Utilities|FlowControl|Delay 0.5)
  (Variables|Default|SetIsTeleporting false)
  (Utilities|FlowControl|Sequence
    (:then_0
      (bind _teleportvfx (Variables|Default|GetTeleportVFX)
        (:then
          (Components|DestroyComponent _teleportvfx))
        (:else)))
    (:then_1
      (bind _trailvfx (Variables|Default|GetTrailVFX)
        (:then
          (Components|DestroyComponent _trailvfx))
        (:else)))))

(event Custom|HealOverTime
  (Animation|Montage|PlayMontage (Variables|Character|GetMesh) "/Game/Enemies/Animation/ProMagic/Standing_2H_Cast_Spell_01_Montage.Standing_2H_Cast_Spell_01_Montage"
    (:OnCompleted
      _)
    (:OnInterrupted
      _))
  (Default|Heal (Variables|Default|GetBPC_Attack) 0.0))

(event EventBeginPlay
  (|CallParentFunction) ; This node is disabled and will not be called.\nDrag off pins to build functionality.
)

(event Collision|EventActorBeginOverlap
  (params (OtherActor :type Actor%20Object%20Reference)))

(event EventTick
  (params (DeltaSeconds :type Float%20%28single-precision%29)))

(fn ConstructionScript
  (|CallParentFunction))