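; Melee enemy Blueprint that adds great sword blocking on top of its parent class.
; StartBlock halts movement, flags the damage system component as blocking and plays the block montage.
; A blocked hit changes BlockingState and plays an impact montage; an interruption in that state ends the block, as does normal montage completion.
; EndBlock clears the flag, resets BlockingState and calls OnBlockEnded.
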(event OnBlocked(BPC_DamageSystem)
  (params (CanBeParried :type Boolean))
  (Variables|Default|SetBlockingState "NewEnumerator2")
  (Animation|Montage|PlayMontage (Variables|Character|GetMesh) "/Game/Enemies/Animation/Sword/MM_Great_Sword_Impact_Anim_Montage.MM_Great_Sword_Impact_Anim_Montage"))

(event Custom|StartBlock
  (Components|Movement|StopMovementImmediately (Variables|Character|GetCharacterMovement))
  (Variables|Default|SetBlockingState "NewEnumerator1")
  (Variables|/Game/DamageSystem/BPC_DamageSystem.BPC_DamageSystem_C|SetIsBlocking (Variables|Default|GetBPC_DamageSystem) true)
  (Animation|Montage|PlayMontage (Variables|Character|GetMesh) "/Game/Enemies/Animation/Sword/MM_Great_Sword_Blocking__1__Anim_Montage.MM_Great_Sword_Blocking__1__Anim_Montage"
    (:OnCompleted
      (CallFunction|EndBlock :!label _label))
    (:OnInterrupted
      (if (Utilities|Enum|Equal(Enum) (Variables|Default|GetBlockingState) "NewEnumerator2")
        (goto _label)))))

(event Custom|EndBlock
  (Variables|/Game/DamageSystem/BPC_DamageSystem.BPC_DamageSystem_C|SetIsBlocking (Variables|Default|GetBPC_DamageSystem) false)
  (Variables|Default|SetBlockingState "NewEnumerator0")
  (Default|CallOnBlockEnded))

(event EventBeginPlay
  (|CallParentFunction))

(event Collision|EventActorBeginOverlap
  (params (OtherActor :type Actor%20Object%20Reference)))

(event EventTick
  (params (DeltaSeconds :type Float%20%28single-precision%29)))

(fn ConstructionScript
  (|CallParentFunction))