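; Base enemy character that takes damage, reacts to hits and ragdolls on death, with a widget health bar.
; Health, healing and damage functions forward to BPCDamageSystem, whose death and damage-response events are bound in the construction script.
; A hit stops movement and sets AIC_EnemyBase to Frozen during the hit montage, then Attack once it completes or is interrupted.
; Death enables mesh physics, stops the AI brain and sets the controller state to Dead.
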(event Custom|OnDeath
  (bind _self self)
  (bind _mesh (Variables|Character|GetMesh))
  (bind _returnvalue (AI|GetAIController _self))
  (Physics|SetSimulatePhysics _mesh true)
  (Collision|SetCollisionEnabled _mesh "QueryAndPhysics")
  (AI|Logic|StopLogic (Variables|/Script/AIModule.AIController|GetBrainComponent _returnvalue) "")
  (bind _asaic_enemy_base (Utilities|Casting|CastToAIC_EnemyBase _returnvalue))
  (Default|SetStateasDead _asaic_enemy_base))

(event Custom|OnDamageResponded
  (params (DamageResponse :type E_DamageResponse%20Enum :default "NewEnumerator0"))
  (Components|Movement|StopMovementImmediately (Variables|Character|GetCharacterMovement))
  (bind _asaic_enemy_base (Utilities|Casting|CastToAIC_EnemyBase (AI|GetAIController self)))
  (Default|SetStateasFrozen _asaic_enemy_base)
  (Animation|Montage|PlayMontage (Variables|Character|GetMesh) (Variables|Default|GetHitMontage) 1.5
    (:OnCompleted
      _)
    (:OnInterrupted
      _))
  (Default|SetStateasAttack _asaic_enemy_base))

(event EventBeginPlay
  (bind _returnvalue (UserInterface|CreateWidget "/Game/DamageSystem/WBP_HealthBar.WBP_HealthBar_C" 0 self))
  (UserInterface|SetWidget (Variables|Default|GetHealthBar) _returnvalue))

(fn ConstructionScript
  (bind _bpc_damagesystem (Variables|Default|GetBPC_DamageSystem))
  (EventDispatchers|BindEventtoOnDeath _bpc_damagesystem (EventDispatchers|CreateEvent :!event Custom|OnDeath))
  (EventDispatchers|BindEventtoOnDamageResponded _bpc_damagesystem (EventDispatchers|CreateEvent :!event Custom|OnDamageResponded)))

(fn GetCurHealth
  (bind _health (Default|GetCurHealth (Variables|Default|GetBPC_DamageSystem)))
  (return _health))

(fn GetMaxHealth
  (bind _maxhealth (Default|GetMaxHealth (Variables|Default|GetBPC_DamageSystem)))
  (return _maxhealth))

(fn Heal
  (params (Amount :type Float%20%28double-precision%29))
  (bind _updatedhealth (Default|Heal (Variables|Default|GetBPC_DamageSystem) Amount))
  (return _updatedhealth))

(fn IsAttacking
  (return (Variables|Default|GetAttacking)))

(fn IsDead
  (return (Variables|/Game/DamageSystem/BPC_DamageSystem.BPC_DamageSystem_C|GetIsDead (Variables|Default|GetBPC_DamageSystem))))

(fn TakeDamage
  (params (DamageInfo :type S%20Damage%20Info%20Structure))
  (bind _wasdamaged (Default|TakeDamage (Variables|Default|GetBPC_DamageSystem) DamageInfo))
  (return _wasdamaged))