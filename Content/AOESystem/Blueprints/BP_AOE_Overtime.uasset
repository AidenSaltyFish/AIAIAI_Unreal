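; BP_AOE_Overtime is an area-of-effect actor that repeatedly applies its effect over a limited lifetime.
; On BeginPlay it attaches an emitter to its root and starts two timers.
; A looping timer fires at ActivateInterval to call SpawnAOESphere, which is not defined in this graph.
; A one-shot timer destroys the actor once Lifetime expires.
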(event Custom|Activate
  (CallFunction|SpawnAOESphere))

(event Custom|Destroy
  (Actor|DestroyActor))

(event EventBeginPlay
  (Effects|SpawnEmitterAttached (Variables|Default|GetEmitter%20Template) (Variables|Default|GetDefaultSceneRoot) "None")
  (Utilities|FlowControl|Sequence
    (:then_0
      (Utilities|Time|SetTimerbyEvent (delegate Custom|Activate) (Variables|Default|GetActivateInterval) true))
    (:then_1
      (Utilities|Time|SetTimerbyEvent (delegate Custom|Destroy) (Variables|Default|GetLifetime)))))

(event Collision|EventActorBeginOverlap
  (params (OtherActor :type Actor%20Object%20Reference)))

(event EventTick
  (params (DeltaSeconds :type Float%20%28single-precision%29)))

(fn ConstructionScript
  (|CallParentFunction))