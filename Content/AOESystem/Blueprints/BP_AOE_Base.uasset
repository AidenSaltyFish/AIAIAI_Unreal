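; BP_AOE_Base is a base area-of-effect actor that finds Pawns within a sphere around its root.
; SpawnAOESphere runs a one-shot sphere overlap query, optionally excluding the instigator, with an optional debug sphere.
; Each hit actor is broadcast through the OnAOEOverlappedActor dispatcher, and the base applies no effect itself.
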(event Custom|SpawnAOESphere
  (bind _defaultsceneroot (Variables|Default|GetDefaultSceneRoot))
  (bind _returnvalue (Transformation|GetWorldLocation _defaultsceneroot))
  (if (Variables|Default|GetDrawDebugSphere)
    (Rendering|Debug|DrawDebugSphere _returnvalue (Variables|Default|GetSphere%20Radius) 12 "(R=0.950915,G=0.000000,B=1.000000,A=1.000000)" 1e+01))
  (bind _outactors (Collision|SphereOverlapActors _returnvalue (Variables|Default|GetSphere%20Radius) (Utilities|Array|MakeArray "ObjectTypeQuery3") 0 (select (Variables|Default|GetIgnoreInstigator) (Utilities|Array|MakeArray (Game|GetInstigator)) 0)))
  (for _array_element _outactors
    (Default|CallOnAOEOverlappedActor _array_element)))

(fn ConstructionScript)