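; Lightning area-of-effect actor that shows a ground warning decal before its strike.
; On BeginPlay it snaps to the floor with a visibility trace, whose end scales Z by -100 rather than subtracting an offset.
; It spawns the decal there and waits TimeBeforeStrike.
; If the decal is still valid, it destroys it and only then calls parent BeginPlay, deferring the inherited behavior until after the warning.
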(event Custom|MoveToFloor
  (bind _target (Variables|Default|GetTarget))
  (bind _returnvalue (Transformation|GetActorLocation _target))
  (bind (_outhit _returnvalue_2) (Collision|LineTraceByChannel _returnvalue (* _returnvalue "1.000000,1.000000,-100.000000") "TraceTypeQuery1" false (Utilities|Array|MakeArray _target) "None"))
  (if _returnvalue_2
    (Transformation|SetActorLocation (.Location (Collision|BreakHitResult _outhit)) false false)))

(event EventBeginPlay
  (CallFunction|MovetoFloor)
  (bind _returnvalue (Rendering|Decal|SpawnDecalatLocation "/Game/Fab/Utility_Marking_Decals/utilityMarkings00.utilityMarkings00" "25.000000,256.000000,256.000000" (Transformation|GetActorLocation) "-90.000000,0.000000,0.000000" 0.0))
  (Utilities|FlowControl|Delay (Variables|Default|GetTimeBeforeStrike))
  (if (Utilities|IsValid _returnvalue)
    (Components|DestroyComponent _returnvalue)
    (|CallParentFunction)))

(event Collision|EventActorBeginOverlap
  (params (OtherActor :type Actor%20Object%20Reference))
  (|CallParentFunction OtherActor) ; This node is disabled and will not be called.\nDrag off pins to build functionality.
)

(event EventTick
  (params (DeltaSeconds :type Float%20%28single-precision%29))
  (|CallParentFunction DeltaSeconds) ; This node is disabled and will not be called.\nDrag off pins to build functionality.
)

(fn ConstructionScript
  (|CallParentFunction))